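; BP_MyCharacter is a player character Blueprint that handles combat feedback and the game-over transition.
; It creates a hidden combo HUD on BeginPlay, which DisplayCombo shows, animates or hides based on CharWeapon's combo count, and spawns animated floating damage text on AnyDamage.
; Tick pins X to ProperX, constraining movement to a plane.
; EndGame flags a loss in the game instance and opens GameOverScreen; pause-menu logic is unconnected.
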(event `InputAction|Pause`
  (params (Key :type "Key Structure")))

(event `self.ReceiveBeginPlay`
  (set `self.IsScreenShow` false)
  (set `self.IsPauseAva` true)
  (bind _returnvalue (`|CreateWidget` "/Game/UI/BP_Combo.BP_Combo_C"))
  (`UserWidget.AddToViewport` _returnvalue 0)
  (bind _output_get (set `self.ComboHUD` _returnvalue))
  (`Widget.SetVisibility` _output_get "Hidden")
  (set `/Game/UI/BP_Combo.Owner` self _output_get))

(event `self.ReceiveTick`
  (params (DeltaSeconds :type "Float (single-precision)"))
  (`self.K2_SetActorLocation` (`KismetMathLibrary.MakeVector` (`self.properX`) (.y (`self.K2_GetActorLocation`)) (.z (`self.K2_GetActorLocation`)))))

(event `self.endGame`
  (bind _asbp_game_instance (cast `/Game/Blueprints/BP_GameInstance` (`GameplayStatics.GetGameInstance`)))
  (set `/Game/Blueprints/BP_GameInstance.PlayerWon` false _asbp_game_instance)
  (`GameplayStatics.OpenLevel` "GameOverScreen"))

(event `self.ReceiveAnyDamage`
  (params (Damage :type "Float (single-precision)") (DamageType :type "DamageType Object Reference") (InstigatedBy :type "Controller Object Reference") (DamageCauser :type "Actor Object Reference"))
  (bind _returnvalue (`|CreateWidget` "/Game/UI/Damage.Damage_C" null self))
  (set `/Game/UI/Damage.Float Damage` Damage _returnvalue)
  (`UserWidget.AddToViewport` _returnvalue 0)
  (`UserWidget.PlayAnimation` _returnvalue (`/Game/UI/Damage.FloatingTextAnim` _returnvalue) 0.0 1 "Forward" 1.0))

(event `self.displayCombo`
  (bind _combohud (`self.ComboHUD`))
  (bind _combohud_2 (`self.ComboHUD`))
  (bind _combohud_3 (`self.ComboHUD`))
  (if (== (`Weapon.comboCount` (`self.CharWeapon`)) 1)
    (`Widget.SetVisibility` _combohud_3 "Visible")
    (`UserWidget.PlayAnimation` _combohud_3 (`/Game/UI/BP_Combo.TransitionIn` _combohud_3) 0.0 1 "Forward" 1.0)
    (elif (== (`Weapon.comboCount` (`self.CharWeapon`)) 0)
      (`UserWidget.PlayAnimation` _combohud (`/Game/UI/BP_Combo.ComboAnimation` _combohud) 0.0 1 "Reverse" 1.0)
      (`KismetSystemLibrary.Delay` 0.3)
      (`Widget.SetVisibility` _combohud "Hidden")
      (elif (>= (`Weapon.comboCount` (`self.CharWeapon`)) 2)
        (`UserWidget.PlayAnimation` _combohud_2 (`/Game/UI/BP_Combo.ComboAnimation` _combohud_2) 0.0 1 "Forward" 1.0)))))

(fn `UserConstructionScript`)