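; HitNotifyState is an animation notify state that marks the hit window inside attack animations.
; On begin, it casts the mesh owner to BP_MyCharacter, or failing that BP_Enemy, and calls StartHit on it, printing a debug string for the player.
; On end, it calls EndHit only on BP_MyCharacter, so enemies receive no matching end call from this notify.
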(fn `Received_NotifyBegin`
  (params (MeshComp :type "SkeletalMeshComponent Object Reference") (Animation :type "AnimSequenceBase Object Reference") (TotalDuration :type "Float (double-precision)"))
  (returns (ReturnValue :type Boolean))
  (bind _returnvalue (`ActorComponent.GetOwner` MeshComp))
  (bind _asbp_my_character (cast `/Game/Blueprints/BP_MyCharacter` _returnvalue)
    (:`then`
      (`KismetSystemLibrary.PrintString` null "player char")
      (`TP_SideScrollerCharacter.StartHit` _asbp_my_character))
    (:`CastFailed`
      (bind _asbp_enemy (cast `/Game/Blueprints/BP_Enemy` _returnvalue))
      (`TP_SideScrollerCharacter.StartHit` _asbp_enemy)))
  (return false))

(fn `Received_NotifyEnd`
  (params (MeshComp :type "SkeletalMeshComponent Object Reference") (Animation :type "AnimSequenceBase Object Reference"))
  (returns (ReturnValue :type Boolean))
  (bind _asbp_my_character (cast `/Game/Blueprints/BP_MyCharacter` (`ActorComponent.GetOwner` MeshComp)))
  (`TP_SideScrollerCharacter.EndHit` _asbp_my_character)
  (return false))