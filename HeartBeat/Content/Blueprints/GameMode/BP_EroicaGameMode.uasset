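; BP_EroicaGameMode is the game mode that sets up the level's HUD and spawns its enemy when play begins.
; It picks a hard-coded enemy spawn transform by checking whether the level is CaveMap, with a fallback location for any other map.
; It creates BP_HUD for the first player, spawns BP_Enemy, and passes that enemy reference to the HUD.
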(event `self.ReceiveBeginPlay`
  (bind _returnvalue (`GameplayStatics.GetCurrentLevelName` true))
  (if (`KismetStringLibrary.EqualEqual_StrStr` _returnvalue "CaveMap")
    (set `self.EnemySpawn` (`KismetMathLibrary.MakeTransform` (500.0 -2900.0 300.0)))
    (else
      (set `self.EnemySpawn` (`KismetMathLibrary.MakeTransform` (230.0 360.0 610.0)))))
  (bind _returnvalue_2 (`|CreateWidget` "/Game/UI/BP_HUD.BP_HUD_C" (`GameplayStatics.GetPlayerController` 0)))
  (`UserWidget.AddToViewport` _returnvalue_2 0)
  (set `self.Level HUD` _returnvalue_2)
  (bind _returnvalue_3 (`|SpawnActorFromClass` "/Game/Blueprints/BP_Enemy.BP_Enemy_C" (`self.EnemySpawn`) "Undefined" "OverrideRootScale" null null))
  (bind _output_get (set `self.EnemyAI` _returnvalue_3))
  (set `/Game/UI/BP_HUD.Enemy` _output_get (`self.Level HUD`)))

(event `self.ReceiveTick`
  (params (DeltaSeconds :type "Float (single-precision)")))

(fn `UserConstructionScript`)