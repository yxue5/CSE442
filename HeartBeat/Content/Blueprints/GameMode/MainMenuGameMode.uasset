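; Game mode for the main menu level, setting up its HUD and a single enemy character.
; On BeginPlay it creates BP_HUD for the first player, adds it to the viewport, spawns BP_Enemy at a fixed location and passes that enemy to the HUD.
; Each tick it polls the I key on the first player controller to toggle the enemy's AI mode flag.
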(event `self.ReceiveBeginPlay`
  (bind _returnvalue (`|CreateWidget` "/Game/UI/BP_HUD.BP_HUD_C" (`GameplayStatics.GetPlayerController` 0)))
  (`UserWidget.AddToViewport` _returnvalue 0)
  (set `self.Level HUD` _returnvalue)
  (bind _returnvalue_2 (`|SpawnActorFromClass` "/Game/Blueprints/BP_Enemy.BP_Enemy_C" (`KismetMathLibrary.MakeTransform` (220.0 360.0 610.0)) "Undefined" "OverrideRootScale" null null))
  (bind _output_get (set `self.Enemy Character` _returnvalue_2))
  (set `/Game/UI/BP_HUD.Enemy` _output_get (`self.Level HUD`)))

(event `self.ReceiveTick`
  (params (DeltaSeconds :type "Float (single-precision)"))
  (bind _enemy_character (`self.Enemy Character`))
  (if (`PlayerController.WasInputKeyJustPressed` (`GameplayStatics.GetPlayerController` 0) "I")
    (if (`AI_Kisa.isAIMode` _enemy_character)
      (set `AI_Kisa.isAIMode` false _enemy_character)
      (else
        (set `AI_Kisa.isAIMode` true _enemy_character)))))

(fn `UserConstructionScript`)