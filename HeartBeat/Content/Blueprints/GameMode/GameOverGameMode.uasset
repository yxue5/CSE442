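; Game mode for the game over screen, which runs all its logic on BeginPlay.
; It spawns two BP_MyCharacter actors as a backdrop, one looping a victory animation and the other playing a defeat animation once, regardless of the result.
; It shows the mouse cursor and adds the GameOver widget with Game and UI input.
; The PlayerWon flag in BP_GameInstance only picks the win or fail sound.
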(event `self.ReceiveBeginPlay`
  (set `PlayerController.bShowMouseCursor` true (`GameplayStatics.GetPlayerController` 0))
  (bind _returnvalue (`|SpawnActorFromClass` "/Game/Blueprints/BP_MyCharacter.BP_MyCharacter_C" (`KismetMathLibrary.MakeTransform` (350.0 400.0 500.0)) "Undefined" "OverrideRootScale" null null))
  (`SkeletalMeshComponent.PlayAnimation` (`Character.Mesh` _returnvalue) "/Game/Art_Assets/Animations/VictoryUnreal_Anim.VictoryUnreal_Anim" true)
  (bind _returnvalue_2 (`|SpawnActorFromClass` "/Game/Blueprints/BP_MyCharacter.BP_MyCharacter_C" (`KismetMathLibrary.MakeTransform` (350.0 -500.0 500.0)) "Undefined" "OverrideRootScale" null null))
  (`SkeletalMeshComponent.PlayAnimation` (`Character.Mesh` _returnvalue_2) "/Game/Art_Assets/Animations/DefeatUnreal_Anim.DefeatUnreal_Anim" false)
  (bind _returnvalue_3 (`|CreateWidget` "/Game/UI/GameOver.GameOver_C"))
  (`UserWidget.AddToViewport` _returnvalue_3 0)
  (`WidgetBlueprintLibrary.SetInputMode_GameAndUIEx` (`GameplayStatics.GetPlayerController` 0) _returnvalue_3)
  (bind _asbp_game_instance (cast `/Game/Blueprints/BP_GameInstance` (`GameplayStatics.GetGameInstance`)))
  (if (`/Game/Blueprints/BP_GameInstance.PlayerWon` _asbp_game_instance)
    (`GameplayStatics.PlaySound2D` "/Game/Maps/Map3_Assets/BGM/Winner_Sound_Effects_Cue.Winner_Sound_Effects_Cue")
    (else
      (`GameplayStatics.PlaySound2D` "/Game/Maps/Map3_Assets/BGM/FAIL_SOUND_EFFECT.FAIL_SOUND_EFFECT"))))

(fn `UserConstructionScript`)