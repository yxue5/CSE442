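; Game mode for the game over screen, announcing whether the player won or lost.
; On BeginPlay it spawns two BP_MyCharacter actors at fixed locations.
; It then reads PlayerWon from BP_GameInstance, prints it, and plays either a winner or a fail sound.
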(event `self.ReceiveBeginPlay`
  (`|SpawnActorFromClass` "/Game/Blueprints/BP_MyCharacter.BP_MyCharacter_C" (`KismetMathLibrary.MakeTransform` (300.0 400.0 500.0)) "Undefined" "OverrideRootScale" null null)
  (`|SpawnActorFromClass` "/Game/Blueprints/BP_MyCharacter.BP_MyCharacter_C" (`KismetMathLibrary.MakeTransform` (300.0 -250.0 500.0)) "Undefined" "OverrideRootScale" null null)
  (bind _asbp_game_instance (cast `/Game/Blueprints/BP_GameInstance` (`GameplayStatics.GetGameInstance`)))
  (bind _playerwon (`/Game/Blueprints/BP_GameInstance.PlayerWon` _asbp_game_instance))
  (`KismetSystemLibrary.PrintString` (`KismetStringLibrary.Conv_BoolToString` _playerwon))
  (if _playerwon
    (`GameplayStatics.PlaySound2D` "/Game/Maps/Map3_Assets/BGM/Winner_Sound_Effects_Cue.Winner_Sound_Effects_Cue")
    (else
      (`GameplayStatics.PlaySound2D` "/Game/Maps/Map3_Assets/BGM/FAIL_SOUND_EFFECT.FAIL_SOUND_EFFECT"))))

(fn `UserConstructionScript`)