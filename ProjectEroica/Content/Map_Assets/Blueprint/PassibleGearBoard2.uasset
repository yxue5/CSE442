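; PassibleGearBoard2 is a gear board Blueprint with a helper for placing a platform on a circle around a gear.
; PlatformRotateAroundGear centers on a valid target actor's location, falling back to the supplied location.
; It rotates a Y-axis radius vector around X by angle plus rotation rate, moves the platform there unswept, and returns the center.
; The function stores no angle and nothing here calls it, so callers must drive the motion.
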(fn `PlatformRotateAroundGear`
  (params (ActorToRotate :type "Actor Object Reference") (TargetActor :type "Actor Object Reference") (targetLocation :type "Vector Structure") (radius :type "Float (double-precision)") (angle :type "Float (double-precision)") (rotationRate :type "Float (double-precision)"))
  (returns (NewParam :type "Vector Structure"))
  (locals (LActorToRotate :type "Actor Object Reference") (LTargetActor :type "Actor Object Reference") (LTargetLocation :type "Vector Structure") (LRadius :type "Float (double-precision)") (LAngle :type "Float (double-precision)") (LRotationRate :type "Float (double-precision)"))
  ;[1 1 1] This function is to set the Target actor and rotate around the target actor.
  (set `local.LActorToRotate` ActorToRotate)
  (set `local.LTargetActor` TargetActor)
  (set `local.LTargetLocation` targetLocation)
  (set `local.LRadius` radius)
  (set `local.LAngle` angle)
  (set `local.LRotationRate` rotationRate)
  (`/Engine/EditorBlueprintResources/StandardMacros.IsValid` (`local.LTargetActor`)
    (:`Is Valid`
      (set `local.LTargetLocation` (`self.K2_GetActorLocation` (`local.LTargetActor`))))
    (:`Is Not Valid`
      _))
  (`self.K2_SetActorLocation` (`local.LActorToRotate`) (+ (`local.LTargetLocation`) (`KismetMathLibrary.RotateAngleAxis` (`KismetMathLibrary.MakeVector` 0.0 (`local.LRadius`)) (+ (`local.LRotationRate`) (`local.LAngle`)) (1.0 0.0 0.0))) false false)
  (return (`local.LTargetLocation`)))

(fn `UserConstructionScript`)