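; Player character Blueprint that handles opening the pause menu and showing floating damage numbers.
; Pause input, gated by IsScreenShow and IsPauseAva, creates the PauseMenu widget, switches to game-and-UI input with a visible cursor and pauses the game.
; AnyDamage creates a Damage widget that references the character, passes in the amount and plays its floating-text animation.
; Tick prints the GetState result every frame as debug output.
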(event `InputAction|Pause`
  (params (Key :type "Key Structure"))
  (bind _returnvalue (`GameplayStatics.GetPlayerController` 0))
  (:`Pressed`
    (if (`self.IsScreenShow`)
      _
      (elif (`self.IsPauseAva`)
        (bind _returnvalue_2 (`|CreateWidget` "/Game/UI/PauseMenu.PauseMenu_C"))
        (`UserWidget.AddToViewport` _returnvalue_2 0)
        (`WidgetBlueprintLibrary.SetInputMode_GameAndUIEx` _returnvalue _returnvalue_2)
        (set `PlayerController.bShowMouseCursor` true _returnvalue)
        (set `self.IsScreenShow` true)
        (`GameplayStatics.SetGamePaused` true)))))

(event `self.ReceiveTick`
  (params (DeltaSeconds :type "Float (single-precision)"))
  (bind _returnvalue (`self.getState`))
  (`KismetSystemLibrary.PrintString` _returnvalue))

(event `self.ReceiveBeginPlay`)

(event `self.ReceiveAnyDamage`
  (params (Damage :type "Float (single-precision)") (DamageType :type "DamageType Object Reference") (InstigatedBy :type "Controller Object Reference") (DamageCauser :type "Actor Object Reference"))
  (bind _returnvalue (`|CreateWidget` "/Game/UI/Damage.Damage_C" null self))
  (set `/Game/UI/Damage.Float Damage` Damage _returnvalue)
  (`UserWidget.AddToViewport` _returnvalue 0)
  (`UserWidget.PlayAnimation` _returnvalue (`/Game/UI/Damage.FloatingTextAnim` _returnvalue) 0.0 1 "Forward" 1.0))

(fn `UserConstructionScript`)